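; BP_CubeProjection is an actor that projects an image onto surrounding scene geometry through a decal scaled by projection distance.
; Its construction script stores the actor's transform in the settings and builds a dynamic M_CubeProjection material with the preview image.
; Optional depth comes from a cube scene capture into a render target created by custom C++.
; SetProjectionTexture recaptures and swaps the image; disconnected examples show UMG and media texture sources.
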(fn `SetProjectionTexture`
  (params (Texture :type "Texture Object Reference"))
  (`SceneCaptureComponentCube.CaptureScene` (`self.SceneCaptureComponentCube`))
  (`MaterialInstanceDynamic.SetTextureParameterValue` (`self.ProjectionMID`) "Image" Texture))

(fn `UpdateProjection`
  (bind _scenecapturecomponentcube (`self.SceneCaptureComponentCube`))
  (bind _scenecapturecomponentcube_2 (`self.SceneCaptureComponentCube`))
  (bind ((`DepthBias_17_0526F894424F344CF062DEAA0CFDC0EF` _depthbias) (`Gamma_18_44EFAA594F569E5DF355BA8602178DD0` _gamma) (`Brightness_19_C7615E844AA35FF983EE9B8586AD00A4` _brightness)) (break `/Projector/CubeProjection/CubeProjectionSettings` (`self.ProjectionSettings`)))
  (setmembers `/Projector/CubeProjection/CubeProjectionSettings` :`StructRef` (`self.ProjectionSettings`) :`ProjectOrigin` (`self.K2_GetActorLocation`) :`ProjectRotator` (`self.K2_GetActorRotation`))
  (`|ExecutionSequence`
    (:`then_0`
      (`SceneComponent.SetWorldScale3D` (`self.Decal`) (`KismetMathLibrary.Conv_DoubleToVector` (`.ProjectDistance_38_A6317325454A3E7AA248029F29849DF9` (break `/Projector/CubeProjection/CubeProjectionSettings` (`self.ProjectionSettings`))))))
    (:`then_1`
      (bind _returnvalue (`KismetMaterialLibrary.CreateDynamicMaterialInstance` "/Projector/CubeProjection/M_CubeProjection.M_CubeProjection"))
      (bind _output_get (set `self.ProjectionMID` _returnvalue))
      (`MaterialInstanceDynamic.SetTextureParameterValue` _output_get "Image" (`self.PreviewImage`))
      (`MaterialInstanceDynamic.SetScalarParameterValue` (`self.ProjectionMID`) "DepthBias" _depthbias)
      (`MaterialInstanceDynamic.SetScalarParameterValue` (`self.ProjectionMID`) "Gamma" _gamma)
      (`MaterialInstanceDynamic.SetScalarParameterValue` (`self.ProjectionMID`) "Brightness" _brightness)
      (`MaterialInstanceDynamic.SetScalarParameterValue` (`self.ProjectionMID`) "EnableDepth" 1.0)
      (`DecalComponent.SetDecalMaterial` (`self.Decal`) (`self.ProjectionMID`)))
    (:`then_2`
      (if (`.bEnableDepth_49_77AA248E4A1FAB3AD9AF8AB22DA97EBD` (break `/Projector/CubeProjection/CubeProjectionSettings` (`self.ProjectionSettings`)))
        (bind _returnvalue_2 (`ProjectorBPLibrary.CreateRenderTargetCube` (`.DepthSize_41_4D03C3BD4162D09E379354A9AF54FD6A` (break `/Projector/CubeProjection/CubeProjectionSettings` (`self.ProjectionSettings`))))) ; 这是一个自定义的C++方法\n用来创建立方体渲染目标\n引擎没有内置的方法
        (bind _output_get_2 (set `SceneCaptureComponentCube.TextureTarget` _returnvalue_2 (`self.SceneCaptureComponentCube`)))
        (`MaterialInstanceDynamic.SetTextureParameterValue` (`self.ProjectionMID`) "Depth" _output_get_2)
        (set `SceneCaptureComponent.bCaptureOnMovement` true _scenecapturecomponentcube)
        (set `SceneCaptureComponent.bCaptureEveryFrame` (`.bUpdateDepthEveryFrame_47_8623FFF540F41B1C98BFD4AE861B2C04` (break `/Projector/CubeProjection/CubeProjectionSettings` (`self.ProjectionSettings`))) _scenecapturecomponentcube)
        (else
          (set `SceneCaptureComponent.bCaptureOnMovement` false _scenecapturecomponentcube_2)
          (set `SceneCaptureComponent.bCaptureEveryFrame` false _scenecapturecomponentcube_2)
          (`MaterialInstanceDynamic.SetScalarParameterValue` (`self.ProjectionMID`) "EnableDepth" 0.0))))))

(fn `UserConstructionScript`
  (`self.UpdateProjection`))