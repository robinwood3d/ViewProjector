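; Projector actor that casts a texture into the scene through a decal, sized by horizontal/vertical FOV and distance.
; Construction runs UpdateProjection, building decal and far-plane material instances and scaling the frustum components.
; Optional depth comes from a SceneCapture2D rendering to an R16f target, captured with a widened FOV and fed to both materials.
; SetProjectionTexture recaptures and swaps the image; unwired examples show widget, render target and media texture sources.
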(event `self.ReceiveBeginPlay`)

(fn `SetProjectionTexture`
  (params (Texture :type "Texture Object Reference"))
  (`SceneCaptureComponent2D.CaptureScene` (`self.SceneCaptureComponent2D`))
  (`MaterialInstanceDynamic.SetTextureParameterValue` (`self.ProjectionMID`) "Image" Texture))

(fn `UpdateProjection`
  (bind _scenecapturecomponent2d (`self.SceneCaptureComponent2D`))
  (bind _scenecapturecomponent2d_2 (`self.SceneCaptureComponent2D`))
  (bind _lineofsight (`self.LineOfSight`))
  (bind ((`DepthSize_47_1B79A5194BFEE79A0BF48E976D5757BC` _depthsize)) (break `/Projector/ViewProjection/FProjectionSettings` (`self.ProjectionSettings`)))
  (bind ((`ProjectDistance_6_F3BF99A0474B43A7D5896F94B0FB28AF` _projectdistance) (`HorizontalFOV_10_2A22BB464C1F0832B4D6A2AD94388461` _horizontalfov) (`VerticalFOV_9_C60EA70447410276E19060918CFC1C1F` _verticalfov)) (break `/Projector/ViewProjection/FProjectionSettings` (`self.ProjectionSettings`)))
  (bind ((`HorizontalFOV_10_2A22BB464C1F0832B4D6A2AD94388461` _horizontalfov_2) (`VerticalFOV_9_C60EA70447410276E19060918CFC1C1F` _verticalfov_2)) (break `/Projector/ViewProjection/FProjectionSettings` (`self.ProjectionSettings`)))
  (bind ((`SphereBlendAlpha_35_1D5251C6473362E55BD4F3B732300251` _sphereblendalpha) (`DepthBias_38_44F543964E9D2F6C5D8E288E99778663` _depthbias) (`Gamma_41_EBF21487402EC69E88511A8643304831` _gamma) (`Brightness_44_49EB21754BCE36953E7065BA21058BA7` _brightness)) (break `/Projector/ViewProjection/FProjectionSettings` (`self.ProjectionSettings`)))
  (bind (_returnvalue_x _returnvalue_y _returnvalue_z) (`KismetMathLibrary.BreakVector` (`SceneComponent.K2_GetComponentScale` (`self.Origin`))))
  (bind _returnvalue (`KismetMathLibrary.DegTan` (* _horizontalfov_2 0.5)))
  (setmembers `/Projector/ViewProjection/FProjectionSettings` :`StructRef` (`self.ProjectionSettings`) :`ProjectOrigin` (`self.K2_GetActorLocation`) :`ProjectRotator` (`self.K2_GetActorRotation`))
  (`|ExecutionSequence`
    (:`then_0`
      (bind _returnvalue_2 (`KismetMaterialLibrary.CreateDynamicMaterialInstance` "/Projector/ViewProjection/Materials/M_ViewProjection.M_ViewProjection"))
      (set `self.ProjectionMID` _returnvalue_2)
      (bind _returnvalue_3 (`PrimitiveComponent.CreateDynamicMaterialInstance` (`self.ViewFarPlane`) 0 "/Projector/ViewProjection/Materials/M_ViewFarPlane.M_ViewFarPlane" "None"))
      (set `self.FarPlaneMID` _returnvalue_3)
      (`MaterialInstanceDynamic.SetTextureParameterValue` (`self.ProjectionMID`) "Image" (`self.PreviewImage`))
      ;[1 0.979 0] 解决远距离出现的条纹
      (`MaterialInstanceDynamic.SetScalarParameterValue` (`self.ProjectionMID`) "DepthBias" _depthbias)
      (`MaterialInstanceDynamic.SetScalarParameterValue` (`self.ProjectionMID`) "Gamma" _gamma)
      (`MaterialInstanceDynamic.SetScalarParameterValue` (`self.ProjectionMID`) "Brightness" _brightness)
      (`MaterialInstanceDynamic.SetScalarParameterValue` (`self.ProjectionMID`) "SphereBlendAlpha" _sphereblendalpha)
      (`MaterialInstanceDynamic.SetScalarParameterValue` (`self.FarPlaneMID`) "SphereBlendAlpha" _sphereblendalpha)
      (`MaterialInstanceDynamic.SetScalarParameterValue` (`self.ProjectionMID`) "EnableDepth" 1.0)
      (`MaterialInstanceDynamic.SetScalarParameterValue` (`self.FarPlaneMID`) "EnableDepth" 1.0)
      (`DecalComponent.SetDecalMaterial` (`self.Decal`) (`self.ProjectionMID`)))
    (:`then_1`
      (if (`.bEnableDepth_51_7EAB4C044884BB8E4620EAB0149AFC4D` (break `/Projector/ViewProjection/FProjectionSettings` (`self.ProjectionSettings`)))
        (set `SceneCaptureComponent2D.FOVAngle` (* (`KismetMathLibrary.DegAtan` (* _returnvalue 2.0)) 2.0) (`self.SceneCaptureComponent2D`))
        (bind _returnvalue_4 (`KismetRenderingLibrary.CreateRenderTarget2D` _depthsize (`KismetMathLibrary.FTrunc` (* _depthsize (/ (`KismetMathLibrary.DegTan` (* _verticalfov_2 0.5)) _returnvalue))) "RTF_R16f"))
        (bind _output_get (set `SceneCaptureComponent2D.TextureTarget` _returnvalue_4 (`self.SceneCaptureComponent2D`)))
        (`MaterialInstanceDynamic.SetTextureParameterValue` (`self.ProjectionMID`) "Depth" _output_get)
        (`MaterialInstanceDynamic.SetTextureParameterValue` (`self.FarPlaneMID`) "Depth" _output_get)
        (set `SceneCaptureComponent.bCaptureOnMovement` true _scenecapturecomponent2d)
        (set `SceneCaptureComponent.bCaptureEveryFrame` (`.bUpdateDepthEveryFrame_49_FD64141A4450C8D116FBD181FF637189` (break `/Projector/ViewProjection/FProjectionSettings` (`self.ProjectionSettings`))) _scenecapturecomponent2d)
        (else
          (set `SceneCaptureComponent.bCaptureOnMovement` false _scenecapturecomponent2d_2)
          (set `SceneCaptureComponent.bCaptureEveryFrame` false _scenecapturecomponent2d_2)
          (`MaterialInstanceDynamic.SetScalarParameterValue` (`self.ProjectionMID`) "EnableDepth" 0.0)
          (`MaterialInstanceDynamic.SetScalarParameterValue` (`self.FarPlaneMID`) "EnableDepth" 0.0))))
    (:`then_2`
      (`SceneComponent.SetRelativeScale3D` (`self.Origin`) (`KismetMathLibrary.MakeVector` _projectdistance (* (`KismetMathLibrary.DegTan` (* _horizontalfov 0.5)) _projectdistance 2.0) (* (`KismetMathLibrary.DegTan` (* _verticalfov 0.5)) _projectdistance 2.0)))
      (`SceneComponent.SetAbsolute` _lineofsight false false true)
      (`SceneComponent.SetAbsolute` (`self.ViewFarPlane`) false false true)
      (`SceneComponent.SetWorldScale3D` _lineofsight (`KismetMathLibrary.MakeVector` (`.ProjectDistance_6_F3BF99A0474B43A7D5896F94B0FB28AF` (break `/Projector/ViewProjection/FProjectionSettings` (`self.ProjectionSettings`))) 0.01 0.01))
      (`SceneComponent.SetWorldScale3D` (`self.ViewFarPlane`) (`KismetMathLibrary.MakeVector` (* _returnvalue_z 2.0) (* _returnvalue_y 2.0) _returnvalue_x))
      (`SceneComponent.SetVisibility` (`self.ViewFarPlane`) (`.bUseFarPlane_29_6360DF1A461BEB087A00A2A177E2544B` (break `/Projector/ViewProjection/FProjectionSettings` (`self.ProjectionSettings`))) false))))

(fn `UserConstructionScript`
  (`self.UpdateProjection`))